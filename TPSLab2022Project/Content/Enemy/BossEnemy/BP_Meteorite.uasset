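; BP_Meteorite is a boss-enemy projectile that launches on BeginPlay and damages the third-person character it overlaps.
; It computes an arcing velocity toward a point Distance ahead along its forward vector and applies it to the physics-driven Sphere.
; Any overlap destroys it, with damage passed through the character's health component.
; Spawn and hit particles and sounds run from event dispatcher bindings, which this graph never broadcasts.
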(event Custom|OnMeteoriteSpawned_Event
  (bind _returnvalue (Transformation|GetActorLocation))
  (Effects|SpawnEmitteratLocation (Variables|Default|GetSpawn%20EFX) _returnvalue)
  (Audio|SpawnSoundatLocation (Variables|Default|GetSpawn%20SFX) _returnvalue "0, 0, 0" 1.0 1.0 0.0 0 0))

(event Custom|OnMeteoriteHit_Event
  (Effects|SpawnEmitteratLocation (Variables|Default|GetHit%20EFX) (Transformation|GetWorldLocation (Variables|Default|GetSphere)))
  (Audio|SpawnSoundatLocation (Variables|Default|GetHit%20SFX) "0, 0, 0" "0, 0, 0" 1.0 1.0 0.0 0 0))

(event EventBeginPlay
  (bind _returnvalue (Transformation|GetActorLocation))
  (EventDispatchers|BindEventtoOnMeteoriteHit (delegate Custom|OnMeteoriteHit_Event))
  (EventDispatchers|AssignOnMeteoriteSpawned (delegate Custom|OnMeteoriteSpawned_Event))
  (bind _outlaunchvelocity (Game|SuggestProjectileVelocityCustomArc _returnvalue (+ (* (Transformation|GetActorForwardVector) (Variables|Default|GetDistance)) _returnvalue) 0.0 0.5))
  (Physics|SetPhysicsLinearVelocity (Variables|Default|GetSphere) _outlaunchvelocity false "None"))

(event Collision|EventActorBeginOverlap
  (params (OtherActor :type Actor%20Object%20Reference))
  (bind _astp_third_person_character (Utilities|Casting|CastToTP_ThirdPersonCharacter OtherActor)
    (:then
      (Class|HealthComponent|GetDamage (Class|TPThirdPersonCharacter|GetHealthComponent _astp_third_person_character) (Variables|Default|GetDamage)))
    (:CastFailed
      _))
  (Actor|DestroyActor))

(fn ConstructionScript)