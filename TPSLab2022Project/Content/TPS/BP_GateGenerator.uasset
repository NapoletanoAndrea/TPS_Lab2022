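; Gate trigger that shuts a gate on the player and reopens it once a linked enemy area is cleared.
; On overlap while open, it clears IsOpen before casting to the third-person character, then a timeline lerps the gate from its BeginPlay location to FinalPoint.
; When EnemyArea updates with no live enemies, a second timeline lerps it back, without resetting IsOpen.
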(event OnAreaUpdated(EnemyArea)
  (params (EnemyArea :type Enemy%20Area%20Object%20Reference))
  (if (not (Class|EnemyArea|ContainsLiveEnemies EnemyArea))
    (bind _t (Timeline|Timeline_0 Play)
      (:Update
        (Transformation|SetActorLocation (Variables|Default|GetGate) (Math|Vector|Lerp(Vector) (Transformation|GetActorLocation (Variables|Default|GetFinalPoint)) (Variables|Default|GetStartLocation) _t) false false)))))

(event EventBeginPlay
  (Variables|Default|SetStartLocation (Transformation|GetActorLocation (Variables|Default|GetGate))))

(event Collision|EventActorBeginOverlap
  (params (OtherActor :type Actor%20Object%20Reference))
  (if (Variables|Default|GetIsOpen)
    (Variables|Default|SetIsOpen false)
    (Utilities|Casting|CastToTP_ThirdPersonCharacter OtherActor)
    (bind _t (Timeline|Timeline Play)
      (:Update
        (Transformation|SetActorLocation (Variables|Default|GetGate) (Math|Vector|Lerp(Vector) (Variables|Default|GetStartLocation) (Transformation|GetActorLocation (Variables|Default|GetFinalPoint)) _t) false false)))))

(event EventTick
  (params (DeltaSeconds :type Float%20%28single-precision%29)))

(fn ConstructionScript)