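; BP_AudioManager is an actor that switches the game's music to match the combat state of the enemies.
; On BeginPlay it finds the EnemyManager, binds to its OnStatusUpdated event and spawns a 2D sound starting with the Stealth track.
; When the status changes, it prints the new state and swaps the audio component to the Stealth, Fighting or Calm cue, restarting playback without a crossfade.
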(event Custom|OnStatusUpdated_Event_0
  (params (CombatStatus :type ECombatStatus%20Enum :default "Stealth") (bStatusChanged :type Boolean))
  (bind _audiocomponent (Variables|Default|GetAudioComponent))
  (if bStatusChanged
    (Development|PrintString (Utilities|String|EnumtoString CombatStatus) true true "(R=0.000000,G=0.660000,B=1.000000,A=1.000000)" 5.0)
    (if (Utilities|Enum|Equal(Enum) CombatStatus "Stealth")
      (Audio|Components|Audio|SetSound _audiocomponent "/Game/Sounds/Stealth_Cue.Stealth_Cue")
      (Audio|Components|Audio|Play _audiocomponent 0.0 :!label _label)
      (elif (Utilities|Enum|Equal(Enum) CombatStatus "Chasing")
        (Audio|Components|Audio|SetSound _audiocomponent "/Game/Sounds/Fighting_Cue.Fighting_Cue")
        (goto _label)
        (elif (Utilities|Enum|Equal(Enum) CombatStatus "Calm")
          (Audio|Components|Audio|SetSound _audiocomponent "/Game/Sounds/Calm_Cue.Calm_Cue")
          (goto _label))))))

(event EventBeginPlay
  (bind _returnvalue (Actor|GetActorOfClass "/Script/UnrealStudies.EnemyManager"))
  (EventDispatchers|AssignOnStatusUpdated _returnvalue (delegate Custom|OnStatusUpdated_Event_0))
  (bind _returnvalue_2 (Audio|SpawnSound2D "/Game/Sounds/Stealth.Stealth" 1.0 1.0 0.0 0))
  (Variables|Default|SetAudioComponent _returnvalue_2))

(fn ConstructionScript)